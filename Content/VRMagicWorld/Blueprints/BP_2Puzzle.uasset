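; BP_2Puzzle is an actor in VRMagicWorld that shuttles back and forth along the world Y axis, likely as a puzzle element.
; The construction script seeds PosInicial with the actor's Y, and each Tick offsets it by Vel, signed by SentidoPositivo, then stores the new Y.
; Crossing RecorridoInicio or RecorridoFinal sets the direction back into range.
; Movement is per frame, without delta-time scaling.
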(event `self.ReceiveTick`
  (params (DeltaSeconds :type "Float (single-precision)"))
  (bind (_returnvalue_x _returnvalue_y) (`KismetMathLibrary.BreakVector` (`self.K2_GetActorLocation`)))
  (bind (_returnvalue_x_2 _returnvalue_y_2 _returnvalue_z) (`KismetMathLibrary.BreakVector` (`self.K2_GetActorLocation`)))
  (bind _vel (`self.vel`))
  (`self.K2_SetActorLocation` (`KismetMathLibrary.MakeVector` _returnvalue_x_2 (+ (`self.PosInicial`) (select `bool` (`self.SentidoPositivo`) :`false` (* _vel -1.0) :`true` _vel)) _returnvalue_z))
  ;[1 1 1] Si posInicial se pasa de rango, cambio el sentido
  (bind _output_get (set `self.PosInicial` _returnvalue_y))
  (`|ExecutionSequence`
    (:`then_0`
      (if (< _output_get (`self.RecorridoInicio`))
        (set `self.SentidoPositivo` true)))
    (:`then_1`
      (if (> _output_get (`self.RecorridoFinal`))
        (set `self.SentidoPositivo` false)))))

(fn `UserConstructionScript`
  (bind (_returnvalue_x _returnvalue_y) (`KismetMathLibrary.BreakVector` (`self.K2_GetActorLocation`)))
  (set `self.PosInicial` _returnvalue_y))