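; VR wand that grabs and carries physics objects from a distance, using a Physics Handle aimed along an Arrow component.
; Tick line-traces forward, highlights components whose actor has AC_PickableObjectM via material swap, and keeps any held object at a fixed distance ahead.
; Trigger press grabs the last hit component with a brief ice-beam effect.
; Release drops it and applies the crate material; unselected highlights are never reset.
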(event `self.ReceiveTick`
  (params (DeltaSeconds :type "Float (single-precision)"))
  (bind _arrow (`self.Arrow`))
  (bind _arrow_2 (`self.Arrow`))
  (bind _returnvalue (`SceneComponent.K2_GetComponentLocation` _arrow_2))
  ;[0.765 0.9498 1] Actualiza en todo momento la pos. del objeto agarrado
  (`|ExecutionSequence`
    (:`then_0`
      (if (`self.CogiendoObjeto`)
        (`PhysicsHandleComponent.SetTargetLocation` (`self.PhysicsHandle`) (+ (`SceneComponent.K2_GetComponentLocation` _arrow) (* (`SceneComponent.GetForwardVector` _arrow) 400.0)))))
    (:`then_1`
      ;[1 0.5809 0.551] Lanza una linea que colisiona con el componente a buscar
      (bind (_outhit _returnvalue_2) (`KismetSystemLibrary.LineTraceSingle` _returnvalue (+ _returnvalue (* (`SceneComponent.GetForwardVector` _arrow_2) 650.0)) "TraceTypeQuery1"))
      (if _returnvalue_2
        (bind (_bblockinghit _binitialoverlap _time _distance _location _impactpoint _normal _impactnormal _physmat _hitactor _hitcomponent) (`GameplayStatics.BreakHitResult` _outhit))
        ;[0.5896 0.8361 1] Cambio el material al simplemente colisionar con el cmp. para señalar que puede agarrarlo
        (`/Engine/EditorBlueprintResources/StandardMacros.IsValid` (`self.GetComponentByClass` _hitactor "/Game/VRMagicWorld/Blueprints/AC_PickableObjectM.AC_PickableObjectM_C")
          (:`Is Valid`
            (bind _output_get (set `self.Hit Component` _hitcomponent))
            (`PrimitiveComponent.SetMaterial` _output_get 0 "/Game/StylizedProvencal/Materials/MI_Ground_VertexPaint.MI_Ground_VertexPaint")
            (set `self.PuedeCogerObjeto` true)))
        (else
          (set `self.PuedeCogerObjeto` false))))))

(event `/Game/VRMagicWorld/Blueprints/BP_VRInteractionBPI.TriggerPressed`
  (bind _arrow (`self.Arrow`))
  (bind _arrow_2 (`self.Arrow`))
  ;[1 0.3926 0.3528] Verifica si puede ser agarrado el cmp y pulsando el trigger del mando lo agarra
  (if (`self.PuedeCogerObjeto`)
    (`PhysicsHandleComponent.GrabComponentAtLocationWithRotation` (`self.PhysicsHandle`) (`self.Hit Component`) "None" (+ (`SceneComponent.K2_GetComponentLocation` _arrow) (* (`SceneComponent.GetForwardVector` _arrow) 400.0)) (struct))
    ;[0.6049 1 0.3695] Creo un trazado de particulas
    (set `self.CogiendoObjeto` true)
    (bind _returnvalue (`GameplayStatics.SpawnEmitterAttached` "/Game/InfinityBladeEffects/Effects/FX_Monsters/FX_Monster_Elemental/ICE/P_Beam_Laser_Ice_Large.P_Beam_Laser_Ice_Large" _arrow_2 "None" (`SceneComponent.K2_GetComponentLocation` _arrow_2) (struct) (0.6 0.6 0.6)))
    (`KismetSystemLibrary.Delay` 0.2)
    (`ActorComponent.K2_DestroyComponent` _returnvalue)))

(event `/Game/VRMagicWorld/Blueprints/BP_VRInteractionBPI.TriggerReleased`
  ;[0.8154 0.9496 1] Al soltar el trigger, suelto el objeto gracias al cmp handle, y vuelvo a poner su material
  (if (`self.CogiendoObjeto`)
    (`PhysicsHandleComponent.ReleaseComponent` (`self.PhysicsHandle`))
    (set `self.CogiendoObjeto` false)
    (`PrimitiveComponent.SetMaterial` (`self.Hit Component`) 0 "/Game/StylizedProvencal/Materials/MI_Crates.MI_Crates")))

(fn `UserConstructionScript`)