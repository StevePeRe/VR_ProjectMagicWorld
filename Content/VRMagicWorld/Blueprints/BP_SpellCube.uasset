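; BP_SpellCube is a spell puzzle cube that shows its collision state with the spell pillar through its material.
; Each Tick polls flags on BPSpellComponent: a lost puzzle resets hit state and restores the base material.
; Otherwise the change-color flag applies the collision material, with the warning flag as fallback for a danger material signalling that the cube can hit the pillar again.
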(event `self.ReceiveTick`
  (params (DeltaSeconds :type "Float (single-precision)"))
  (bind _bp_spellcomponent (`self.BP_SpellComponent`))
  (bind _cube (`self.Cube`))
  (bind _bp_spellcomponent_2 (`self.BP_SpellComponent`))
  ;[1 1 1] Reset de valores
  (if (`/Game/VRMagicWorld/Blueprints/AC_SpellComponent.LosePuzzle` _bp_spellcomponent)
    (set `/Game/VRMagicWorld/Blueprints/AC_SpellComponent.CanHit` true _bp_spellcomponent_2)
    (set `/Game/VRMagicWorld/Blueprints/AC_SpellComponent.LosePuzzle` false _bp_spellcomponent_2)
    (set `/Game/VRMagicWorld/Blueprints/AC_SpellComponent.hits` 0 _bp_spellcomponent_2)
    (`PrimitiveComponent.SetMaterial` (`self.Cube`) 0 "/Game/VRMagicWorld/Materials/M_BaseColorSpell.M_BaseColorSpell")
    (else
      ;[1 1 1] Cambiar color al colisionar con pilar del hechizo
      (if (`/Game/VRMagicWorld/Blueprints/AC_SpellComponent.ChangeColor` _bp_spellcomponent)
        (`PrimitiveComponent.SetMaterial` _cube 0 "/Game/VRMagicWorld/Materials/M_ChangeColor.M_ChangeColor")
        (else
          ;[1 1 1] Cambiar a color Peligro ya que puede colisionar otra vez con el pilar
          (if (`/Game/VRMagicWorld/Blueprints/AC_SpellComponent.ChangeWarningColor` _bp_spellcomponent)
            (`PrimitiveComponent.SetMaterial` _cube 0 "/Game/InfinityBladeEffects/Effects/FX_Materials/Misc/M_Bubbles_Set_01_SubUV_INST.M_Bubbles_Set_01_SubUV_INST")))))))

(fn `UserConstructionScript`)